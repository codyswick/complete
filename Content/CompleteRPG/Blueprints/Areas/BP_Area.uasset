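; BP_Area is a world map area that players discover by entering it and that tracks completion of its actor-based tasks.
; Two radius-scaled spheres set compass zone states, including for mounted horse riders, with danger states only in dangerous areas.
; Discovery grants XP, shows a popup and clears markers.
; Discovery and task progress pass through Server-to-All events and update the map widgets, including an eagle-event overlay.
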(event OnComponentEndOverlap(CasualZone)
  (params (OverlappedComponent :type Primitive%20Component%20Object%20Reference) (OtherActor :type Actor%20Object%20Reference) (OtherComp :type Primitive%20Component%20Object%20Reference) (OtherBodyIndex :type Integer))
  ;[1 1 1] Overlap Events
  ;;[1 1 1] On Casual zone overlap
  (CallFunction|HorseEvent OtherActor "NewEnumerator4")
  (Utilities|IsValid (Actor|GetComponentbyClass OtherActor "/Game/CompleteRPG/Blueprints/MapComponents/WorldMap/AC_WorldMap.AC_WorldMap_C")
    (:Is%20Valid
      (CallFunction|ChangeCompassState OtherActor "NewEnumerator4"))))

(event OnComponentBeginOverlap(DangerousZone)
  (params (OverlappedComponent :type Primitive%20Component%20Object%20Reference) (OtherActor :type Actor%20Object%20Reference) (OtherComp :type Primitive%20Component%20Object%20Reference) (OtherBodyIndex :type Integer) (bFromSweep :type Boolean) (SweepResult :type Hit%20Result%20Structure%20%28by%20ref%29))
  ;[1 1 1] Overlap Events
  ;;[1 1 1] Dangerous Zone Overlap
  (CallFunction|HorseEvent OtherActor "NewEnumerator2")
  (Utilities|IsValid (Actor|GetComponentbyClass OtherActor "/Game/CompleteRPG/Blueprints/MapComponents/WorldMap/AC_WorldMap.AC_WorldMap_C")
    (:Is%20Valid
      (CallFunction|ChangeCompassState OtherActor "NewEnumerator2"))))

(event OnComponentBeginOverlap(CasualZone)
  (params (OverlappedComponent :type Primitive%20Component%20Object%20Reference) (OtherActor :type Actor%20Object%20Reference) (OtherComp :type Primitive%20Component%20Object%20Reference) (OtherBodyIndex :type Integer) (bFromSweep :type Boolean) (SweepResult :type Hit%20Result%20Structure%20%28by%20ref%29))
  ;[1 1 1] Overlap Events
  ;;[1 1 1] On Casual zone overlap
  (Actor|SetOwner OtherActor)
  (CallFunction|HorseEvent OtherActor "NewEnumerator1")
  (CallFunction|AreaDiscovered-Server OtherActor))

(event OnComponentEndOverlap(DangerousZone)
  (params (OverlappedComponent :type Primitive%20Component%20Object%20Reference) (OtherActor :type Actor%20Object%20Reference) (OtherComp :type Primitive%20Component%20Object%20Reference) (OtherBodyIndex :type Integer))
  (bind _returnvalue (Actor|GetComponentbyClass OtherActor "/Game/CompleteRPG/Blueprints/MapComponents/WorldMap/AC_WorldMap.AC_WorldMap_C"))
  ;[1 1 1] Overlap Events
  ;;[1 1 1] Dangerous Zone Overlap
  (CallFunction|HorseEvent _returnvalue "NewEnumerator3")
  (Utilities|IsValid _returnvalue
    (:Is%20Valid
      (CallFunction|ChangeCompassState OtherActor "NewEnumerator3"))))

(event Custom|UpateArea
  ;[1 1 1] Update The Area
  (Utilities|Struct|SetmembersinS_AreaStateStat (Variables|/Game/CompleteRPG/UI/Widgets/WorldMap/WorldPlace/WB_MapArea.WB_MapArea_C|GetAreaInfo (Variables|Default|GetWB_Area))))

(event Custom|AddTaskToDone%20-Server
  (params (Actor :type Object%20Object%20Reference))
  ;[1 1 1] Area Multiplayer
  (CallFunction|AddTasktoDone-ALL Actor))

(event Custom|AddTaskToDone%20-ALL
  (params (Actor :type Object%20Object%20Reference))
  (bind _areainfo (Variables|Default|GetAreaInfo))
  (bind _areainfo_2 (Variables|Default|GetAreaInfo))
  (bind (_area _discovered_ _tasks _donetasks) (Utilities|Struct|BreakS_AreaStateStat _areainfo))
  ;[1 1 1] Write area tasks progress
  (bind (_array_index _array_element) (CallFunction|GetTaskbyActorReference _tasks Actor))
  (bind _output_get (Variables|Default|SetHoldDoneTasks _donetasks))
  (bind _output_get_2 (Variables|Default|SetHoldDoneActors (.Actors (Utilities|Struct|BreakS_pTaskList (Utilities|Array|Get(acopy) _output_get _array_index)))))
  (Utilities|Array|Add _output_get_2 _array_element)
  (bind _structout (Utilities|Struct|SetmembersinS_pTaskList (Utilities|Array|Get(acopy) _output_get _array_index) (Variables|Default|GetHoldDoneActors)))
  (Utilities|Array|SetArrayElem (Variables|Default|GetHoldDoneTasks) _array_index _structout)
  (Utilities|Struct|SetmembersinS_AreaStateStat (Variables|Default|GetAreaInfo) (Variables|Default|GetHoldDoneTasks))
  (Default|SetNewAreaInfo (Variables|Default|GetWB_Area) _areainfo_2 true)
  (Default|SetNewAreaInfo (CallFunction|GetMapArea) _areainfo_2 false))

(event Custom|TryAddTask
  (params (Actor :type Actor%20Object%20Reference))
  ;[1 1 1] Area Multiplayer
  (Actor|SetOwner Actor)
  (CallFunction|AddTasktoDone-Server Actor))

(event Custom|AreaDiscovered%20-Server
  (params (Object :type Object%20Object%20Reference))
  ;[1 1 1] Overlap Events
  ;;[1 1 1] On Casual zone overlap
  (CallFunction|AreaDiscovered-ALL Object))

(event Custom|EagleEvent
  (bind _aswb_map_area (CallFunction|GetMapArea))
  ;[1 1 1] Eagle Events
  (Variables|/Game/CompleteRPG/UI/Widgets/WorldMap/WorldPlace/WB_MapArea.WB_MapArea_C|SetMapRef _aswb_map_area (Variables|Default|GetMapRef))
  (Variables|/Game/CompleteRPG/UI/Widgets/WorldMap/WorldPlace/WB_MapArea.WB_MapArea_C|SetLocation _aswb_map_area (Transformation|GetActorLocation))
  (Rendering|SetVisibility (Variables|Default|GetAreaWidget) true false))

(event Custom|EagleReversedEvent
  ;[1 1 1] Eagle Events
  (Rendering|SetVisibility (Variables|Default|GetAreaWidget) false false))

(event Custom|AreaDiscovered%20-ALL
  (params (Object :type Object%20Object%20Reference))
  (bind _areainfo (Variables|Default|GetAreaInfo))
  (bind _wb_area (Variables|Default|GetWB_Area))
  (bind _area (Utilities|Struct|BreakS_AreaStateStat _areainfo))
  (bind _output_get (CallFunction|GetAreaInfo _area))
  (bind (_name _hiddenicon _observericon _descoverpoints) (Utilities|Struct|BreakS_AreaInfoStat _output_get))
  ;[1 1 1] Overlap Events
  ;;[1 1 1] On Casual zone overlap
  (bind _ascharacter (Utilities|Casting|CastToCharacter Object))
  (Utilities|IsValid (Actor|GetComponentbyClass _ascharacter "/Game/CompleteRPG/Blueprints/MapComponents/WorldMap/AC_WorldMap.AC_WorldMap_C")
    (:Is%20Valid
      (bind _output_get_2 (Variables|Default|SetOverlapedChaarcter _ascharacter))
      (CallFunction|ChangeCompassState _output_get_2 "NewEnumerator1")
      (Utilities|IsAlreadyDescovered
        (:else
          (CallFunction|RemoveMarker)
          (Utilities|Struct|SetmembersinS_AreaStateStat _areainfo true)
          (Utilities|IsValid (CallFunction|GetCharacterCompass (Variables|Default|GetOverlapedChaarcter))
            (:Is%20Valid
              (Default|Recreate (CallFunction|GetCharacterCompass (Variables|Default|GetOverlapedChaarcter))))
            (:Is%20Not%20Valid
              _))
          (bind _returnvalue (UserInterface|CreateWidget "/Game/CompleteRPG/UI/Widgets/AnnounceScreen/WB_NewArea.WB_NewArea_C" 0 _name _descoverpoints))
          (Default|AddExp (Actor|GetComponentbyClass (Variables|Default|GetOverlapedChaarcter) "/Game/CompleteRPG/Blueprints/MapComponents/PlayerState/AC_ExpSystem.AC_ExpSystem_C") (Math|Conversions|ToFloat(Integer) _descoverpoints))
          (Utilities|IsValid _wb_area
            (:Is%20Valid
              (Utilities|Struct|SetmembersinS_AreaStateStat (Variables|/Game/CompleteRPG/UI/Widgets/WorldMap/WorldPlace/WB_MapArea.WB_MapArea_C|GetAreaInfo _wb_area) true))
            (:Is%20Not%20Valid
              _))
          (UserInterface|Viewport|AddtoViewport _returnvalue 0)
          (Default|SetNewAreaInfo (CallFunction|GetMapArea) (Variables|Default|GetAreaInfo) false))
        (:true
          (CallFunction|RemoveMarker))))))

(event EventBeginPlay
  ;[1 1 1] Area initialization
  (Variables|Default|SetisRuntime true)
  (Rendering|SetVisibility (Variables|Default|GetAreaWidget) false false)
  (Variables|/Game/CompleteRPG/UI/Widgets/WorldMap/WorldPlace/WB_MapArea.WB_MapArea_C|SetAreaInfo (CallFunction|GetMapArea) (Variables|Default|GetAreaInfo))
  (for _array_element (.Tasks (Utilities|Struct|BreakS_AreaStateStat (Variables|Default|GetAreaInfo)))
    (for _array_element_2 (.Actors (Utilities|Struct|BreakS_pTaskList _array_element))
      (bind _asbp_interact_actor (Utilities|Casting|CastToBP_InteractActor _array_element_2))
      (Variables|/Game/CompleteRPG/Blueprints/InteractActors/BP_InteractActor.BP_InteractActor_C|SetAreaReference _asbp_interact_actor self))))

(fn ConstructionScript
  (bind _areainfo (Variables|Default|GetAreaInfo))
  (bind (_area _discovered_ _tasks _donetasks) (Utilities|Struct|BreakS_AreaStateStat _areainfo))
  (|CallParentFunction)
  (Components|Sphere|SetSphereRadius (Variables|Default|GetDangerousZone) (* (Variables|Default|GetSphereRadius) 0.65) true)
  (Components|Sphere|SetSphereRadius (Variables|Default|GetCasualZone) (Variables|Default|GetSphereRadius) false)
  (if (not (Variables|Default|GetisRuntime))
    (Utilities|Array|Clear _donetasks)
    (for _array_element _tasks
      (Utilities|Array|Add _donetasks (Utilities|Struct|MakeS_pTaskList (.Task (Utilities|Struct|BreakS_pTaskList _array_element)) (LocalVariables|GetNoArray))))))

(fn GetTaskbyActorReference
  (params (Array :type Array%20of%20S%20P%20Task%20List%20Structures) (InputPin :type Object%20Object%20Reference))
  (for (_array_element _array_index) Array
    (for _array_element_2 (.Actors (Utilities|Struct|BreakS_pTaskList _array_element))
      (if (== _array_element_2 InputPin)
        (return _array_index _array_element_2))))
  (Development|PrintString "No such actor in tasks! 
" true true "(R=1.000000,G=0.166003,B=0.000000,A=1.000000)" 5.0))

(fn GetMapArea
  (bind _aswb_map_area (Utilities|Casting|CastToWB_MapArea (UserInterface|GetUserWidgetObject (Variables|Default|GetAreaWidget))))
  (return _aswb_map_area))

(fn ChangeCompassState
  (params (Object :type Object%20Object%20Reference) (Zine :type E_ZoneType%20Enum :default "NewEnumerator1"))
  (bind _areainfo (Variables|Default|GetAreaInfo))
  (bind _area (Utilities|Struct|BreakS_AreaStateStat _areainfo))
  (bind _output_get (CallFunction|GetAreaInfo _area))
  (bind (_name _hiddenicon _observericon _descoverpoints _description _dangerous) (Utilities|Struct|BreakS_AreaInfoStat _output_get))
  (Utilities|IsValid Object
    (:Is%20Valid
      (bind _ascharacter (Utilities|Casting|CastToCharacter Object))
      (if _dangerous
        (Utilities|IsValid (CallFunction|GetCharacterCompass _ascharacter)
          (:Is%20Valid
            (Default|NewCompassStatus (CallFunction|GetCharacterCompass _ascharacter) Zine)))
        (else
          (Utilities|IsValid (CallFunction|GetCharacterCompass _ascharacter)
            (:Is%20Valid
              (switch Utilities|FlowControl|Switch|SwitchonE_ZoneType Zine
                (:NewEnumerator1
                  (Default|NewCompassStatus (CallFunction|GetCharacterCompass _ascharacter) "NewEnumerator5"))
                (:NewEnumerator4
                  (Default|NewCompassStatus (CallFunction|GetCharacterCompass _ascharacter) "NewEnumerator6")))))))
      (Variables|/Game/CompleteRPG/UI/Widgets/Compas/WB_Compass.WB_Compass_C|SetAreaName (CallFunction|GetCharacterCompass _ascharacter) _name))))

(fn RemoveMarker
  (if (Variables|/Game/CompleteRPG/UI/Widgets/WorldMap/WorldPlace/WB_MapArea.WB_MapArea_C|GetPlayerMarked (CallFunction|GetMapArea))
    (Default|ToggleMarker (Variables|Default|GetWB_Area))))

(fn HorseEvent
  (params (Object :type Object%20Object%20Reference) (Zine :type E_ZoneType%20Enum :default "NewEnumerator1"))
  (bind _asbp_horse (Utilities|Casting|CastToBP_Horse Object))
  (if (Variables|/Game/CompleteRPG/Horse/Animations/BP_Horse.BP_Horse_C|GetControlled? _asbp_horse)
    (Utilities|IsValid (Variables|/Game/CompleteRPG/Horse/Animations/BP_Horse.BP_Horse_C|GetRememberCharacter _asbp_horse)
      (:Is%20Valid
        (Utilities|IsValid (Actor|GetComponentbyClass (Variables|/Game/CompleteRPG/Horse/Animations/BP_Horse.BP_Horse_C|GetRememberCharacter _asbp_horse) "/Game/CompleteRPG/Blueprints/MapComponents/WorldMap/AC_WorldMap.AC_WorldMap_C")
          (:Is%20Valid
            (CallFunction|ChangeCompassState (Variables|/Game/CompleteRPG/Horse/Animations/BP_Horse.BP_Horse_C|GetRememberCharacter _asbp_horse) Zine)))))))