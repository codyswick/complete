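; BP_ArmorHelper displays equipped inventory items on its owning character through per-slot static and skeletal mesh components.
; On BeginPlay it sets the owner's mesh as master pose for its skeletal meshes.
; AddNewItem and TakeItemOff switch on item subtype to set or clear meshes, preferring skeletal over static and attaching to item-defined sockets.
; It also updates combat weapon state, sets the crossbow anim owner and enables weapon physics on death.
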(event Custom|Attach_Socket_0
  (params (Target :type Scene%20Component%20Object%20Reference))
  ;[1 1 1] Attach First Socket
  (if (Utilities|Name|NotEqual(Name) (Variables|Default|GetSocket) "None")
    _
    (else
      _))
  (Transformation|AttachComponentToComponent Target (Variables|Default|GetPlayerMesh) (Variables|Default|GetSocket) "KeepRelative" "KeepRelative" "KeepRelative" true))

(event Custom|AddNewItem
  (params (Item :type S%20Items%20Inventory%20Dynam%20Structure))
  (CallFunction|AddNewItemF Item)
  (CallFunction|Update))

(event Custom|Attach_Socket_1
  (params (Target :type Scene%20Component%20Object%20Reference))
  ;[1 1 1] Attach Second Socket
  (if (Utilities|Name|NotEqual(Name) (Variables|Default|GetSocket_1) "None")
    (Transformation|AttachComponentToComponent Target (Variables|Default|GetPlayerMesh) (Variables|Default|GetSocket_1) "SnapToTarget" "KeepRelative" "KeepRelative" true)
    (else
      (bind _asskeletal_mesh_component (Utilities|Casting|CastToSkeletalMeshComponent Target))
      (Class|SkinnedMeshComponent|SetSkeletalMesh _asskeletal_mesh_component 0 true))))

(event Custom|TakeItemOff
  (params (Item :type S%20Items%20Inventory%20Dynam%20Structure))
  ;[1 1 1] Take Meshes or Skeletal Mesh off
  (switch Utilities|FlowControl|Switch|SwitchonE_ItemSubtype (.Subtype (Utilities|Struct|BreakS_ItemInvStatic (CallFunction|GetItemInfo (.Item (Utilities|Struct|BreakS_ItemsInventoryDynam Item)))))
    (:NewEnumerator0
      (CallFunction|RemoveMeshfromSlot (Variables|Default|GetFirstWeaponSkeletalMesh) (Variables|Default|GetFirstWeaponStaticMesh) (Variables|Default|GetSecondWeaponSkeletalMesh) (Variables|Default|GetSecondWeaponStaticMesh))
      (bind _asbp_combat_character (Utilities|Casting|CastToBP_CombatCharacter (Variables|Default|GetCharacter)))
      (if (and (Variables|/Game/DynamicCombatSystem/Blueprints/BP_CombatCharacter.BP_CombatCharacter_C|GetIsInCombat _asbp_combat_character) (Utilities|Enum|Equal(Enum) (Variables|/Game/DynamicCombatSystem/Blueprints/BP_CombatCharacter.BP_CombatCharacter_C|GetCombatType _asbp_combat_character) "NewEnumerator1"))
        (Default|PutWeaponBack (Variables|/Game/DynamicCombatSystem/Blueprints/BP_CombatCharacter.BP_CombatCharacter_C|GetAC_Inventory _asbp_combat_character))
        (Variables|/Game/DynamicCombatSystem/Blueprints/BP_CombatCharacter.BP_CombatCharacter_C|SetCombatType _asbp_combat_character "NewEnumerator0")))
    (:NewEnumerator1
      (CallFunction|RemoveMeshfromSlot (Variables|Default|GetCrossbowSkeletalMesh) (Variables|Default|GetCrossbowStaticMesh)))
    (:NewEnumerator2
      (CallFunction|RemoveMeshfromSlot (Variables|Default|GetArrowSkeletalMesh) (Variables|Default|GetArrowStaticMesh)))
    (:NewEnumerator5
      (CallFunction|RemoveMeshfromSlot (Variables|Default|GetTorchSkeletalMesh) (Variables|Default|GetTorchStaticMesh)))
    (:NewEnumerator6
      (CallFunction|RemoveMeshfromSlot (Variables|Default|GetBodySkeletalMesh) (Variables|Default|GetBodyStaticMesh)))
    (:NewEnumerator7
      (CallFunction|RemoveMeshfromSlot (Variables|Default|GetHandsSkeletalMesh_0) (Variables|Default|GetHandsStaticMesh_0) (Variables|Default|GetHandsSkeletalMesh_1) (Variables|Default|GetHandsStaticMesh_1)))
    (:NewEnumerator8
      (CallFunction|RemoveMeshfromSlot (Variables|Default|GetLegsSkeletalMesh_0) (Variables|Default|GetLegsStaticMesh_0) (Variables|Default|GetLegsSkeletalMesh_1) (Variables|Default|GetLegsStaticMesh_1)))
    (:NewEnumerator9
      (CallFunction|RemoveMeshfromSlot (Variables|Default|GetHeadSkeletalMesh) (Variables|Default|GetHeadStaticMesh)))
    (:NewEnumerator11
      (CallFunction|RemoveMeshfromSlot (Variables|Default|GetBagSkeletalMesh) (Variables|Default|GetBagStaticMesh)))
    (:NewEnumerator16
      (CallFunction|RemoveMeshfromSlot (Variables|Default|GetRingSkeletalMeshLeft) (Variables|Default|GetRingStaticMeshLeft)))
    (:NewEnumerator17
      (CallFunction|RemoveMeshfromSlot (Variables|Default|GetAmuletSkeletalMesh) (Variables|Default|GetAmuletStaticMesh)))
    (:NewEnumerator30
      (CallFunction|RemoveMeshfromSlot (Variables|Default|GetShieldSkeletalMesh) (Variables|Default|GetShieldStaticMesh))
      (bind _asbp_combat_character_2 (Utilities|Casting|CastToBP_CombatCharacter (Variables|Default|GetCharacter)))
      (Variables|/Game/DynamicCombatSystem/Blueprints/BP_CombatCharacter.BP_CombatCharacter_C|SetIsShieldEquipped _asbp_combat_character_2 false))
    (:NewEnumerator31
      (CallFunction|RemoveMeshfromSlot (Variables|Default|GetPantsSkeletalMesh) (Variables|Default|GetPantsStaticMesh)))))

(event Custom|SimulateOnDeath
  ;[1 1 1] Simulate Physics
  (Physics|SetSimulatePhysics (Variables|Default|GetFirstWeaponStaticMesh) true))

(event Custom|Update)

(event EventBeginPlay
  (CallFunction|SetPlayerMesh)
  (Utilities|IsValid (Variables|Default|GetPlayerMesh)
    (:Is%20Valid
      (Class|SkinnedMeshComponent|SetMasterPoseComponent (Actor|GetComponentsByClass "/Script/Engine.SkeletalMeshComponent") (Variables|Default|GetPlayerMesh) true))))

(fn ConstructionScript)

(fn AddNewItemF
  (params (S_ItemsInventory :type S%20Items%20Inventory%20Dynam%20Structure%20%28by%20ref%29))
  (bind _item (Utilities|Struct|BreakS_ItemsInventoryDynam S_ItemsInventory))
  (bind _output_get (CallFunction|GetItemInfo _item))
  (bind (_name _description _usagetype _itemtype _rarity _alchemytype _subtype _skilltype _weapontype _reqlevel _class _handssocket _backsocket _picture _weapon_ _mesh _skeletalmesh) (Utilities|Struct|BreakS_ItemInvStatic _output_get))
  (Variables|Default|SetSetNewMesh _mesh)
  (Variables|Default|SetSetNewSkeletalMesh _skeletalmesh)
  (Variables|Default|SetSocket _handssocket)
  (Variables|Default|SetSocket_1 _backsocket)
  (switch Utilities|FlowControl|Switch|SwitchonE_ItemSubtype _subtype
    (:NewEnumerator0
      (Utilities|SelectWeapon
        (:BothWeaponValid
          (CallFunction|SetSubtypeMeshFirstSocket (Variables|Default|GetFirstWeaponStaticMesh) (Variables|Default|GetFirstWeaponSkeletalMesh) :!label _label))
        (:FirstWeaponNotValid
          (goto _label))
        (:SecondWeaponNotValid
          (CallFunction|SetSubtypeMeshFirstSocket (Variables|Default|GetSecondWeaponStaticMesh) (Variables|Default|GetSecondWeaponSkeletalMesh))))
      (bind _asbp_combat_character (Utilities|Casting|CastToBP_CombatCharacter (Components|GetOwner)))
      (if (and (Variables|/Game/DynamicCombatSystem/Blueprints/BP_CombatCharacter.BP_CombatCharacter_C|GetIsInCombat _asbp_combat_character) (Utilities|Enum|Equal(Enum) (Variables|/Game/DynamicCombatSystem/Blueprints/BP_CombatCharacter.BP_CombatCharacter_C|GetCombatType _asbp_combat_character) "NewEnumerator1"))
        (Default|TakeWeapon (CallFunction|GetInventory _asbp_combat_character))))
    (:NewEnumerator1
      (CallFunction|SetSubtypeMeshFirstSocket (Variables|Default|GetCrossbowStaticMesh) (Variables|Default|GetCrossbowSkeletalMesh))
      (CallFunction|SetCrossbowOnner))
    (:NewEnumerator2
      (CallFunction|SetSubtypeMeshFirstSocket (Variables|Default|GetArrowStaticMesh) (Variables|Default|GetArrowSkeletalMesh)))
    (:NewEnumerator5
      (CallFunction|SetSubtypeMeshFirstSocket (Variables|Default|GetTorchStaticMesh) (Variables|Default|GetTorchSkeletalMesh)))
    (:NewEnumerator6
      (CallFunction|SetSubtypeMeshFirstSocket (Variables|Default|GetBodyStaticMesh) (Variables|Default|GetBodySkeletalMesh)))
    (:NewEnumerator7
      (CallFunction|SetSubtypeMeshX2 (Variables|Default|GetHandsStaticMesh_0) (Variables|Default|GetHandsStaticMesh_1) (Variables|Default|GetHandsSkeletalMesh_1) (Variables|Default|GetHandsSkeletalMesh_0)))
    (:NewEnumerator8
      (CallFunction|SetSubtypeMeshX2 (Variables|Default|GetLegsStaticMesh_0) (Variables|Default|GetLegsStaticMesh_1) (Variables|Default|GetLegsSkeletalMesh_1) (Variables|Default|GetLegsSkeletalMesh_0)))
    (:NewEnumerator9
      (CallFunction|SetSubtypeMeshFirstSocket (Variables|Default|GetHeadStaticMesh) (Variables|Default|GetHeadSkeletalMesh)))
    (:NewEnumerator11
      (CallFunction|SetSubtypeMeshFirstSocket (Variables|Default|GetBagStaticMesh) (Variables|Default|GetBagSkeletalMesh)))
    (:NewEnumerator16
      (if (or (Utilities|IsValid (Variables|/Script/Engine.StaticMeshComponent|GetStaticMesh (Variables|Default|GetRingStaticMeshLeft))) (Utilities|IsValid (Variables|/Script/Engine.SkinnedMeshComponent|GetSkeletalMesh (Variables|Default|GetRingSkeletalMeshLeft))))
        (CallFunction|SetSubtypeMeshSecondSocket (Variables|Default|GetRingStaticMeshRight) (Variables|Default|GetRingSkeletalMeshRight))
        (else
          (CallFunction|SetSubtypeMeshFirstSocket (Variables|Default|GetRingStaticMeshLeft) (Variables|Default|GetRingSkeletalMeshLeft)))))
    (:NewEnumerator17
      (CallFunction|SetSubtypeMeshFirstSocket (Variables|Default|GetAmuletStaticMesh) (Variables|Default|GetAmuletSkeletalMesh)))
    (:NewEnumerator30
      (CallFunction|SetSubtypeMeshFirstSocket (Variables|Default|GetShieldStaticMesh) (Variables|Default|GetShieldSkeletalMesh))
      (bind _asbp_combat_character_2 (Utilities|Casting|CastToBP_CombatCharacter (Components|GetOwner)))
      (if (and (Variables|/Game/DynamicCombatSystem/Blueprints/BP_CombatCharacter.BP_CombatCharacter_C|GetIsInCombat _asbp_combat_character_2) (Utilities|Enum|Equal(Enum) (Variables|/Game/DynamicCombatSystem/Blueprints/BP_CombatCharacter.BP_CombatCharacter_C|GetCombatType _asbp_combat_character_2) "NewEnumerator1"))
        (Default|TakeWeapon (CallFunction|GetInventory _asbp_combat_character_2))))
    (:NewEnumerator31
      (CallFunction|SetSubtypeMeshFirstSocket (Variables|Default|GetPantsStaticMesh) (Variables|Default|GetPantsSkeletalMesh)))))

(fn FirstWeaponValid
  (return (or (Utilities|IsValid (Variables|Default|GetFirstWeaponStaticMesh)) (Utilities|IsValid (Variables|Default|GetFirstWeaponSkeletalMesh)))))

(fn SecondWeaponValid
  (return (or (Utilities|IsValid (Variables|Default|GetSecondWeaponSkeletalMesh)) (Utilities|IsValid (Variables|Default|GetSecondWeaponStaticMesh)))))

(fn SetSubtypeMeshFirstSocket
  (params (StaticMesh :type Static%20Mesh%20Component%20Object%20Reference) (SkeletalMesh :type Skeletal%20Mesh%20Component%20Object%20Reference))
  (LocalVariables|SetL_StaticMeshComp StaticMesh)
  (LocalVariables|SetL_SkeletalMeshComponent SkeletalMesh)
  (Utilities|IsValid (Variables|Default|GetSetNewSkeletalMesh)
    (:Is%20Valid
      (Class|SkinnedMeshComponent|SetSkeletalMesh (LocalVariables|GetL_SkeletalMeshComponent) (Variables|Default|GetSetNewSkeletalMesh) true)
      (CallFunction|AttachSocket0 (LocalVariables|GetL_SkeletalMeshComponent)))
    (:Is%20Not%20Valid
      (Utilities|IsValid (Variables|Default|GetSetNewMesh)
        (:Is%20Valid
          (Components|StaticMesh|SetStaticMesh (LocalVariables|GetL_StaticMeshComp) (Variables|Default|GetSetNewMesh))
          (CallFunction|AttachSocket0 (LocalVariables|GetL_StaticMeshComp)))))))

(fn SetSubtypeMeshX2
  (params (StaticMesh_0 :type Static%20Mesh%20Component%20Object%20Reference) (StaticMesh_1 :type Static%20Mesh%20Component%20Object%20Reference) (SkeletalMesh_0 :type Skeletal%20Mesh%20Component%20Object%20Reference) (SkeletalMesh_1 :type Skeletal%20Mesh%20Component%20Object%20Reference))
  (LocalVariables|SetL_StaticMeshComp StaticMesh_0)
  (LocalVariables|SetL_StaticMeshComp_1 StaticMesh_1)
  (LocalVariables|SetL_SkeletalMeshComponent SkeletalMesh_0)
  (LocalVariables|SetL_SkeletalMeshComp_1 SkeletalMesh_1)
  (Utilities|IsValid (Variables|Default|GetSetNewSkeletalMesh)
    (:Is%20Valid
      (Class|SkinnedMeshComponent|SetSkeletalMesh (LocalVariables|GetL_SkeletalMeshComponent) (Variables|Default|GetSetNewSkeletalMesh) true)
      (CallFunction|AttachSocket0 (LocalVariables|GetL_SkeletalMeshComponent))
      (CallFunction|AttachSocket1 (LocalVariables|GetL_SkeletalMeshComp_1)))
    (:Is%20Not%20Valid
      (Utilities|IsValid (Variables|Default|GetSetNewMesh)
        (:Is%20Valid
          (Components|StaticMesh|SetStaticMesh (LocalVariables|GetL_StaticMeshComp) (Variables|Default|GetSetNewMesh))
          (Components|StaticMesh|SetStaticMesh (LocalVariables|GetL_StaticMeshComp_1) (Variables|Default|GetSetNewMesh))
          (CallFunction|AttachSocket0 (LocalVariables|GetL_StaticMeshComp))
          (CallFunction|AttachSocket1 (LocalVariables|GetL_StaticMeshComp_1)))))))

(fn RemoveMeshfromSlot
  (params (SkeletalMesh_0 :type Skinned%20Mesh%20Component%20Object%20Reference) (StaticMesh_0 :type Static%20Mesh%20Component%20Object%20Reference) (SkeletalMesh_1 :type Skinned%20Mesh%20Component%20Object%20Reference) (StaticMesh_1 :type Static%20Mesh%20Component%20Object%20Reference))
  (LocalVariables|SetL_SkeletalMesh_0 SkeletalMesh_0)
  (LocalVariables|SetL_SkeletalMesh_1 SkeletalMesh_1)
  (LocalVariables|SetL_StaticMesh_0 StaticMesh_0)
  (LocalVariables|SetL_StaticMesh_1 StaticMesh_1)
  (Utilities|FlowControl|Sequence
    (:then_0
      (Utilities|IsValid (LocalVariables|GetL_SkeletalMesh_0)
        (:Is%20Valid
          (Class|SkinnedMeshComponent|SetSkeletalMesh (LocalVariables|GetL_SkeletalMesh_0) 0 true))))
    (:then_1
      (Utilities|IsValid (LocalVariables|GetL_SkeletalMesh_1)
        (:Is%20Valid
          (Class|SkinnedMeshComponent|SetSkeletalMesh (LocalVariables|GetL_SkeletalMesh_1) 0 true))))
    (:then_2
      (Utilities|IsValid (LocalVariables|GetL_StaticMesh_0)
        (:Is%20Valid
          (Components|StaticMesh|SetStaticMesh (LocalVariables|GetL_StaticMesh_0) 0))))
    (:then_3
      (Utilities|IsValid (LocalVariables|GetL_StaticMesh_1)
        (:Is%20Valid
          (Components|StaticMesh|SetStaticMesh (LocalVariables|GetL_StaticMesh_1) 0))))))

(fn SetSubtypeMeshSecondSocket
  (params (StaticMesh :type Static%20Mesh%20Component%20Object%20Reference) (SkeletalMesh :type Skeletal%20Mesh%20Component%20Object%20Reference))
  (LocalVariables|SetL_StaticMeshComp StaticMesh)
  (LocalVariables|SetL_SkeletalMeshComponent SkeletalMesh)
  (Utilities|IsValid (Variables|Default|GetSetNewSkeletalMesh)
    (:Is%20Valid
      (Class|SkinnedMeshComponent|SetSkeletalMesh (LocalVariables|GetL_SkeletalMeshComponent) (Variables|Default|GetSetNewSkeletalMesh) true)
      (CallFunction|AttachSocket1 (LocalVariables|GetL_SkeletalMeshComponent)))
    (:Is%20Not%20Valid
      (Utilities|IsValid (Variables|Default|GetSetNewMesh)
        (:Is%20Valid
          (Components|StaticMesh|SetStaticMesh (LocalVariables|GetL_StaticMeshComp) (Variables|Default|GetSetNewMesh))
          (CallFunction|AttachSocket1 (LocalVariables|GetL_StaticMeshComp)))))))

(fn GetMeshbySlot
  (params (Type :type E_ItemSubtype%20Enum :default "NewEnumerator15"))
  (return (Utilities|Select :Index Type :NewEnumerator15 0 :NewEnumerator0 (Variables|Default|GetFirstWeaponSkeletalMesh) :NewEnumerator1 (Variables|Default|GetCrossbowSkeletalMesh) :NewEnumerator2 (Variables|Default|GetArrowSkeletalMesh) :NewEnumerator12 0 :NewEnumerator3 0 :NewEnumerator4 0 :NewEnumerator5 (Variables|Default|GetTorchSkeletalMesh) :NewEnumerator6 (Variables|Default|GetBodySkeletalMesh) :NewEnumerator7 (Variables|Default|GetHandsSkeletalMesh_0) :NewEnumerator8 (Variables|Default|GetLegsSkeletalMesh_0) :NewEnumerator9 (Variables|Default|GetHeadSkeletalMesh) :NewEnumerator10 0 :NewEnumerator11 (Variables|Default|GetBagSkeletalMesh) :NewEnumerator13 0 :NewEnumerator16 (Variables|Default|GetRingSkeletalMeshRight) :NewEnumerator17 (Variables|Default|GetAmuletSkeletalMesh) :NewEnumerator19 (Variables|Default|GetSecondWeaponSkeletalMesh) :NewEnumerator20 0 :NewEnumerator21 (Variables|Default|GetRingSkeletalMeshLeft) :NewEnumerator23 0 :NewEnumerator24 0 :NewEnumerator25 0 :NewEnumerator26 0 :NewEnumerator27 0 :NewEnumerator28 0 :NewEnumerator29 0 :NewEnumerator30 0 :NewEnumerator31 0 :NewEnumerator32 0 :NewEnumerator33 0) (Utilities|Select :Index Type :NewEnumerator15 0 :NewEnumerator0 (Variables|Default|GetFirstWeaponStaticMesh) :NewEnumerator1 (Variables|Default|GetCrossbowStaticMesh) :NewEnumerator2 (Variables|Default|GetArrowStaticMesh) :NewEnumerator12 0 :NewEnumerator3 0 :NewEnumerator4 0 :NewEnumerator5 (Variables|Default|GetTorchStaticMesh) :NewEnumerator6 (Variables|Default|GetBodyStaticMesh) :NewEnumerator7 (Variables|Default|GetHandsStaticMesh_0) :NewEnumerator8 (Variables|Default|GetLegsStaticMesh_0) :NewEnumerator9 (Variables|Default|GetHeadStaticMesh) :NewEnumerator10 0 :NewEnumerator11 (Variables|Default|GetBagStaticMesh) :NewEnumerator13 0 :NewEnumerator16 (Variables|Default|GetRingStaticMeshRight) :NewEnumerator17 (Variables|Default|GetAmuletStaticMesh) :NewEnumerator19 (Variables|Default|GetSecondWeaponStaticMesh) :NewEnumerator20 0 :NewEnumerator21 (Variables|Default|GetRingStaticMeshLeft) :NewEnumerator23 0 :NewEnumerator24 0 :NewEnumerator25 0 :NewEnumerator26 0 :NewEnumerator27 0 :NewEnumerator28 0 :NewEnumerator29 0 :NewEnumerator30 0 :NewEnumerator31 0 :NewEnumerator32 0 :NewEnumerator33 0)))

(fn SetPlayerMesh
  (bind _returnvalue (Components|GetOwner))
  (bind _ascharacter (Utilities|Casting|CastToCharacter _returnvalue)
    (:then
      (bind _output_get (Variables|Default|SetCharacter _ascharacter))
      (Variables|Default|SetPlayerMesh (Variables|/Script/Engine.Character|GetMesh _output_get)))
    (:CastFailed
      (Variables|Default|SetPlayerMesh (Actor|GetComponentbyClass _returnvalue "/Script/Engine.SkeletalMeshComponent")))))

(fn SetCrossbowOnner
  (bind _ascharacter (Utilities|Casting|CastToCharacter (Components|GetOwner)))
  (Class|ICombatState|SetAnimBPOwner(Message) (Components|SkeletalMesh|GetAnimInstance (Variables|Default|GetCrossbowSkeletalMesh)) _ascharacter))