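; Actor component that turns a character's head left or right in its animation instance, following turn input for players or a follow actor for non-players.
; Each tick it interpolates head rotation toward clamped left/right targets derived from mouse, gamepad or look-at yaw.
; The head returns to base when player speed is too low or a non-player lacks a target.
; It also sets the movement yaw rate and can be toggled on or off.
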(event Custom|DeactivateHead
  ;[1 1 1] Toggle Head Active
  (Variables|Default|SetActive? false)
  (Class|BPIHeadRotation|SetHeadRotation(Message) (Variables|Default|GetAnimationInstance) 0.0)
  (Class|BPIHeadRotation|ToggleActive(Message) (Variables|Default|GetAnimationInstance) false))

(event Custom|ActivateHead
  ;[1 1 1] Toggle Head Active
  (Variables|Default|SetActive? true)
  (Class|BPIHeadRotation|ToggleActive(Message) (Variables|Default|GetAnimationInstance) true))

(event Custom|SetTurnRate
  (params (AxisValue :type Float%20%28single-precision%29))
  ;[1 1 1] Get Mouse TurnRate aprox degree
  (Variables|Default|SetTurnRate (* AxisValue 27.0)))

(event EventBeginPlay
  ;[1 1 1] Initialize Component
  (CallFunction|InitializeVariables)
  (CallFunction|SetRotationRate))

(event EventTick
  (params (DeltaSeconds :type Float%20%28single-precision%29))
  ;[1 1 1] Disable head rotation when not moving
  (if (Variables|Default|GetActive?)
    (Utilities|FlowControl|Sequence
      (:then_0
        (bind _value (Class|BPIHeadRotation|GetHeadRotation(Message) (Variables|Default|GetAnimationInstance)))
        (Variables|Default|SetAnimInstanceHeadRotation _value)
        (if (CallFunction|CanRotate?)
          (Utilities|SelectWay
            (:0
              ;[1 1 1] Keep Head Back when not moving
              (CallFunction|SetBaseRotation))
            (:>
              ;[1 1 1] Interpolate the current head rotation to the target rotation
              (Class|BPIHeadRotation|SetHeadRotation(Message) (Variables|Default|GetAnimationInstance) (Math|Interpolation|FInterptoConstant (Variables|Default|GetAnimInstanceHeadRotation) (Variables|Default|GetHeadRotation_R) (Utilities|Time|GetWorldDeltaSeconds) (Variables|Default|GetHeadTurnSpeed))))
            (:<
              (Class|BPIHeadRotation|SetHeadRotation(Message) (Variables|Default|GetAnimationInstance) (Math|Interpolation|FInterptoConstant (Variables|Default|GetAnimInstanceHeadRotation) (* (Variables|Default|GetHeadRotation_L) -1.0) (Utilities|Time|GetWorldDeltaSeconds) (Variables|Default|GetHeadTurnSpeed)))))
          (else
            (CallFunction|SetBaseRotation))))
      (:then_1
        (CallFunction|SetTurnRateCalculation)))))

(fn InitializeVariables
  (bind _ascharacter (Utilities|Casting|CastToCharacter (Components|GetOwner)))
  (bind _output_get (Variables|Default|SetCharacter _ascharacter))
  (Variables|Default|SetAnimationInstance (Components|SkeletalMesh|GetAnimInstance (Variables|/Script/Engine.Character|GetMesh _output_get)))
  (bind _asplayer_controller (Utilities|Casting|CastToPlayerController (Pawn|GetController (Variables|Default|GetCharacter))))
  (Variables|Default|SetPlayerController _asplayer_controller))

(fn SetRotationRate
  (Variables|/Script/Engine.CharacterMovementComponent|SetRotationRate (Variables|/Script/Engine.Character|GetCharacterMovement (Variables|Default|GetCharacter)) (Math|Rotator|MakeRotator 0.0 0.0 (Variables|Default|GetMaxRotation_Z))))

(fn SetTurnRateCalculation
  (bind _yaw (CallFunction|GetDeltaRootationFollowActor))
  (bind _gamepadturnrate (Variables|Default|GetGamepadTurnRate))
  (bind _mousecontrolonly_ (Variables|Default|GetMouseControlOnly?))
  (bind _motionrangemulti_wasd_gpad (Variables|Default|GetMotionRangeMulti_WASD/Gpad))
  (bind _motionrangemulti_mouse (Variables|Default|GetMotionRangeMulti_Mouse))
  (bind _turnrate (Variables|Default|GetTurnRate))
  (bind _returnvalue (* _motionrangemulti_mouse _turnrate))
  (bind _returnvalue_2 (* _motionrangemulti_wasd_gpad -1.0))
  (bind _returnvalue_3 (* _gamepadturnrate _returnvalue_2))
  (bind _returnvalue_4 (select _mousecontrolonly_ _returnvalue _returnvalue_3))
  (Utilities|IsValid (Variables|Default|GetFollowActor)
    (:Is%20Valid
      (Variables|Default|SetHeadRotation_R (Math|Float|Clamp(Float) _yaw 1.0 (Variables|Default|GetHeadMaxRotationDesired_R)))
      (Variables|Default|SetHeadRotation_L (Math|Float|Clamp(Float) (* -1.0 _yaw) 1.0 (Variables|Default|GetHeadMaxRotationDesired_L))))
    (:Is%20Not%20Valid
      (Variables|Default|SetHeadRotation_R (Math|Float|Clamp(Float) (* 1.0 _returnvalue_4) 1.0 (Variables|Default|GetHeadMaxRotationDesired_R)))
      (Variables|Default|SetHeadRotation_L (Math|Float|Clamp(Float) (* -1.0 _returnvalue_4) 1.0 (Variables|Default|GetHeadMaxRotationDesired_L))))))

(fn CanRotate?
  (if (Pawn|IsPlayerControlled (Variables|Default|GetCharacter))
    (return (> (Math|Vector|VectorLength (Transformation|GetComponentVelocity (Variables|/Script/Engine.Character|GetCapsuleComponent (Variables|Default|GetCharacter)))) (Variables|Default|GetGetMinSpeed)))
    (else
      (return (Utilities|IsValid (Variables|Default|GetFollowActor))))))

(fn SetBaseRotation
  (Class|BPIHeadRotation|SetHeadRotation(Message) (Variables|Default|GetAnimationInstance) (Math|Interpolation|FInterptoConstant (Variables|Default|GetAnimInstanceHeadRotation) (Variables|Default|GetHeadRotationBase) (Utilities|Time|GetWorldDeltaSeconds) (Variables|Default|GetHeadTurnSpeed))))

(fn GetDeltaRootationFollowActor
  (bind _followactor (Variables|Default|GetFollowActor))
  (Utilities|IsValid _followactor
    (:Is%20Valid
      (return (- (.Yaw (Math|Rotator|BreakRotator (Math|Rotator|FindLookatRotation (Transformation|GetActorLocation (Variables|Default|GetCharacter)) (Transformation|GetActorLocation _followactor)))) (.Yaw (Math|Rotator|BreakRotator (Transformation|GetActorRotation (Variables|Default|GetCharacter)))))))
    (:Is%20Not%20Valid
      (return 0.0))))