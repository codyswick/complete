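; Actor component that tracks the characters, creatures and books the player has discovered and keeps them in a save game.
; BeginPlay loads the three arrays from a BP_Save_Characters slot, and SaveCharacters writes them back, creating the save object if none exists.
; Add functions skip invalid or duplicate data table rows (matched by row name), append new entries with Discovered false, then refresh the matching info widget through the owner's AC_MainWidgetHandler.
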(event EventBeginPlay
  ;[1 1 1] At the start of the game you load every information you have collected in the game process
  (CallFunction|LoadCharacters))

(fn SaveCharacters
  (bind _returnvalue (SaveGame|DoesSaveGameExist (Variables|Default|GetCharactersSaveSlot)))
  (if _returnvalue
    (bind _returnvalue_2 (SaveGame|LoadGamefromSlot (Variables|Default|GetCharactersSaveSlot)))
    (bind _asbp_save_characters (Utilities|Casting|CastToBP_Save_Characters _returnvalue_2))
    (Variables|Default|SetSaveGAme _asbp_save_characters)
    (else
      (bind _returnvalue_3 (SaveGame|CreateSaveGameObject "/Game/CompleteRPG/Blueprints/Information/CharactersInfo/BP_Save_Characters.BP_Save_Characters_C"))
      (Variables|Default|SetSaveGAme _returnvalue_3)))
  (Variables|/Game/CompleteRPG/Blueprints/Information/CharactersInfo/BP_Save_Characters.BP_Save_Characters_C|SetsCharacters (Variables|Default|GetSaveGAme) (Variables|Default|GetDiscoveredCharacters))
  (Variables|/Game/CompleteRPG/Blueprints/Information/CharactersInfo/BP_Save_Characters.BP_Save_Characters_C|SetsCreatures (Variables|Default|GetSaveGAme) (Variables|Default|GetDiscoveredCreatures))
  (Variables|/Game/CompleteRPG/Blueprints/Information/CharactersInfo/BP_Save_Characters.BP_Save_Characters_C|SetsBooks (Variables|Default|GetSaveGAme) (Variables|Default|GetDiscoveredBooks))
  (SaveGame|SaveGametoSlot (Variables|Default|GetSaveGAme) (Variables|Default|GetCharactersSaveSlot)))

(fn LoadCharacters
  (bind _returnvalue (SaveGame|DoesSaveGameExist (Variables|Default|GetCharactersSaveSlot)))
  (if _returnvalue
    (bind _returnvalue_2 (SaveGame|LoadGamefromSlot (Variables|Default|GetCharactersSaveSlot)))
    (bind _asbp_save_characters (Utilities|Casting|CastToBP_Save_Characters _returnvalue_2))
    (Variables|Default|SetDiscoveredCharacters (Variables|/Game/CompleteRPG/Blueprints/Information/CharactersInfo/BP_Save_Characters.BP_Save_Characters_C|GetsCharacters _asbp_save_characters))
    (Variables|Default|SetDiscoveredCreatures (Variables|/Game/CompleteRPG/Blueprints/Information/CharactersInfo/BP_Save_Characters.BP_Save_Characters_C|GetsCreatures _asbp_save_characters))
    (Variables|Default|SetDiscoveredBooks (Variables|/Game/CompleteRPG/Blueprints/Information/CharactersInfo/BP_Save_Characters.BP_Save_Characters_C|GetsBooks _asbp_save_characters))))

(fn AddNewCharacter
  (params (Character :type Data%20Table%20Row%20Handle%20Structure))
  (bind (_datatable _rowname) (Utilities|Struct|BreakDataTableRowHandle Character))
  (Utilities|IsValid _datatable
    (:Is%20Valid
      (for _array_element (Variables|Default|GetDiscoveredCharacters)
        (if (Utilities|Name|Equal(Name) (.RowName (Utilities|Struct|BreakDataTableRowHandle (.Character (Utilities|Struct|BreakS_CharacterDynam _array_element)))) _rowname)
          (return)))
      (Utilities|Array|Add (Variables|Default|GetDiscoveredCharacters) (Utilities|Struct|MakeS_CharacterDynam Character false))
      (Default|Update (.WB_CharacterInfoWidget (Default|GetWidgets (Actor|GetComponentbyClass (Components|GetOwner) "/Game/CompleteRPG/Blueprints/WidgetHandler/AC_MainWidgetHandler.AC_MainWidgetHandler_C")))))))

(fn TrytoAddABook
  (params (Item :type S%20Items%20Inventory%20Dynam%20Structure))
  (bind _item (Utilities|Struct|BreakS_ItemsInventoryDynam Item))
  (bind _output_get (CallFunction|GetItemInfo _item))
  (bind _bookinfo (Utilities|Struct|BreakS_ItemInvStatic _output_get))
  (Utilities|IsValid (.DataTable (Utilities|Struct|BreakDataTableRowHandle _bookinfo))
    (:Is%20Valid
      (if (not (CallFunction|HasSameBook? _bookinfo))
        (Utilities|Array|Add (Variables|Default|GetDiscoveredBooks) (Utilities|Struct|MakeS_BookDynamic _bookinfo false))
        (Default|Update (Variables|/Game/CompleteRPG/UI/Widgets/Menu/WB_MainGameplayMenu.WB_MainGameplayMenu_C|GetWB_BookInfoWidget (Variables|/Game/CompleteRPG/UI/Widgets/Menu/WB_MainGUI.WB_MainGUI_C|GetWB_MainGameplayMenu (Variables|/Game/CompleteRPG/Blueprints/WidgetHandler/AC_MainWidgetHandler.AC_MainWidgetHandler_C|GetWB_MainGUI (Actor|GetComponentbyClass (Components|GetOwner) "/Game/CompleteRPG/Blueprints/WidgetHandler/AC_MainWidgetHandler.AC_MainWidgetHandler_C")))))))))

(fn HasSameBook?
  (params (Book :type Data%20Table%20Row%20Handle%20Structure%20%28by%20ref%29))
  (for _array_element (Variables|Default|GetDiscoveredBooks)
    (if (Utilities|Name|Equal(Name) (.RowName (Utilities|Struct|BreakDataTableRowHandle (.BookInfo (Utilities|Struct|BreakS_BookDynamic _array_element)))) (.RowName (Utilities|Struct|BreakDataTableRowHandle Book)))
      (return true)))
  (return false))

(fn AddNewCreature
  (params (Creature :type Data%20Table%20Row%20Handle%20Structure))
  (bind (_datatable _rowname) (Utilities|Struct|BreakDataTableRowHandle Creature))
  (Utilities|IsValid _datatable
    (:Is%20Valid
      (for _array_element (Variables|Default|GetDiscoveredCreatures)
        (if (Utilities|Name|Equal(Name) (.RowName (Utilities|Struct|BreakDataTableRowHandle (.Creature (Utilities|Struct|BreakS_CreatureDynamic _array_element)))) _rowname)
          (return)))
      (Utilities|Array|Add (Variables|Default|GetDiscoveredCreatures) (Utilities|Struct|MakeS_CreatureDynamic Creature false))
      (Default|Update (.WB_CreatureInfoWidget (Default|GetWidgets (Actor|GetComponentbyClass (Components|GetOwner) "/Game/CompleteRPG/Blueprints/WidgetHandler/AC_MainWidgetHandler.AC_MainWidgetHandler_C")))))))