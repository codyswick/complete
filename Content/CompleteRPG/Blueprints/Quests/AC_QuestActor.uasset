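; Actor component that holds a quest and reward for its owning actor, such as a quest giver.
; Getters expose the quest, reward and owner, while GiveQuest marks the quest as taken and RefreshQuest replaces it and clears that flag.
; HasTask checks that the quest's data table reference is valid.
; Persistence is unfinished: BeginPlay loads and casts the save slot without applying data, and SaveActor is empty.
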(event EventBeginPlay
  ;[1 1 1] Load Actor
  (CallFunction|LoadActor))

(fn GetQuestandReward
  (return (Variables|Default|GetCurrentQuest) (Variables|Default|GetReward)))

(fn GetQuestandActor
  (return (Variables|Default|GetCurrentQuest) (Components|GetOwner)))

(fn SetMapReference
  (params (Map :type AC%20World%20Map%20Object%20Reference))
  (Variables|Default|SetMap Map))

(fn HasTask
  (return (Utilities|IsValid (.DataTable (Utilities|Struct|BreakDataTableRowHandle (.Quest (Utilities|Struct|BreakS_QuestDynam (Variables|Default|GetCurrentQuest))))))))

(fn GiveQuest
  (Variables|Default|SetActorTookQuest true)
  (return (Variables|Default|GetCurrentQuest)))

(fn RefreshQuest
  (params (CurrentQuest :type S%20Quest%20Dynam%20Structure))
  (Variables|Default|SetCurrentQuest CurrentQuest)
  (Variables|Default|SetActorTookQuest false)
  (return))

(fn SaveActor)

(fn LoadActor
  (bind _returnvalue (SaveGame|DoesSaveGameExist (Variables|Default|GetQuestActor)))
  (if _returnvalue
    (bind _returnvalue_2 (SaveGame|LoadGamefromSlot (Variables|Default|GetQuestActor)))
    (Utilities|Casting|CastToBP_Save_Quests _returnvalue_2)))