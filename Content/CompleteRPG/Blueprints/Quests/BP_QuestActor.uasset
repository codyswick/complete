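; BP_QuestActor is a world quest marker that advances a character's quest when they enter its sphere.
; Construction copies its Quest into ACQuestActor, and shortly after BeginPlay it builds marked-area info from its tracked or untracked state.
; On overlap, it takes the character as owner and checks their AC_QuestsHandler for the same quest exactly one subtask behind.
; A match sets the new subtask with its reward and recreates the character's compass.
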(event OnComponentBeginOverlap(Sphere)
  (params (OverlappedComponent :type Primitive%20Component%20Object%20Reference) (OtherActor :type Actor%20Object%20Reference) (OtherComp :type Primitive%20Component%20Object%20Reference) (OtherBodyIndex :type Integer) (bFromSweep :type Boolean) (SweepResult :type Hit%20Result%20Structure%20%28by%20ref%29))
  (bind _ac_questactor (Variables|Default|GetAC_QuestActor))
  (bind _currentquest (Variables|/Game/CompleteRPG/Blueprints/Quests/AC_QuestActor.AC_QuestActor_C|GetCurrentQuest _ac_questactor))
  (bind (_quest _marked _discovered _currentsubtask) (Utilities|Struct|BreakS_QuestDynam _currentquest))
  ;[1 1 1] Multiplayered Overlap
  (bind _ascharacter (Utilities|Casting|CastToCharacter OtherActor))
  (Utilities|IsValid (Actor|GetComponentbyClass _ascharacter "/Game/CompleteRPG/Blueprints/MapComponents/AC_QuestsHandler.AC_QuestsHandler_C")
    (:Is%20Valid
      (Actor|SetOwner _ascharacter)
      (bind (_found _currentsubtask_2) (CallFunction|SameQuest (Actor|GetComponentbyClass _ascharacter "/Game/CompleteRPG/Blueprints/MapComponents/AC_QuestsHandler.AC_QuestsHandler_C")))
      (if (and _found (== _currentsubtask_2 (- (.CurrentSubTask (Utilities|Struct|BreakS_QuestDynam (Variables|/Game/CompleteRPG/Blueprints/Quests/AC_QuestActor.AC_QuestActor_C|GetCurrentQuest (Variables|Default|GetAC_QuestActor)))) 1)))
        (Default|SetNewQuestSubslot (Actor|GetComponentbyClass _ascharacter "/Game/CompleteRPG/Blueprints/MapComponents/AC_QuestsHandler.AC_QuestsHandler_C") _quest _currentsubtask (Variables|/Game/CompleteRPG/Blueprints/Quests/AC_QuestActor.AC_QuestActor_C|GetReward (Variables|Default|GetAC_QuestActor)))
        ;;[1 1 1] Recreate Compass
        (Default|Recreate (CallFunction|GetCharacterCompass _ascharacter))))))

(event Custom|ChangeState
  (Variables|Default|SetAreaInfo (CallFunction|GetUpdatedMarkedAreaInfo)))

(event EventBeginPlay
  (Utilities|FlowControl|Delay 0.5)
  (CallFunction|ChangeState))

(fn ConstructionScript
  (|CallParentFunction)
  (Variables|/Game/CompleteRPG/Blueprints/Quests/AC_QuestActor.AC_QuestActor_C|SetCurrentQuest (Variables|Default|GetAC_QuestActor) (Variables|Default|GetQuest)))

(fn GetUpdatedMarkedAreaInfo
  (return (Utilities|Struct|MakeS_AreaStateStat (select (Variables|Default|GetActive?) (Variables|Default|GetTrackedTaskInfo) (Variables|Default|GetUntrackedTaskInfo)) true (Utilities|Array|MakeArray "") (Utilities|Array|MakeArray "") (Utilities|Array|MakeArray ""))))

(fn SameQuest
  (params (Character :type AC%20Quests%20Handler%20Object%20Reference))
  (for _array_element (Variables|/Game/CompleteRPG/Blueprints/MapComponents/AC_QuestsHandler.AC_QuestsHandler_C|GetQuests Character)
    (if (Utilities|Name|Equal(Name) (.RowName (Utilities|Struct|BreakDataTableRowHandle (.Quest (Utilities|Struct|BreakS_QuestDynam _array_element)))) (.RowName (Utilities|Struct|BreakDataTableRowHandle (.Quest (Utilities|Struct|BreakS_QuestDynam (Variables|/Game/CompleteRPG/Blueprints/Quests/AC_QuestActor.AC_QuestActor_C|GetCurrentQuest (Variables|Default|GetAC_QuestActor)))))))
      (return true (.CurrentSubTask (Utilities|Struct|BreakS_QuestDynam _array_element)))))
  (return false 0))

(fn HasPrevQuest
  (bind _returnvalue (Actor|GetComponentbyClass "/Game/CompleteRPG/Blueprints/MapComponents/AC_QuestsHandler.AC_QuestsHandler_C"))
  (bind _outputpin (Default|FindQuest _returnvalue (.Quest (Utilities|Struct|BreakS_QuestDynam (Variables|/Game/CompleteRPG/Blueprints/Quests/AC_QuestActor.AC_QuestActor_C|GetCurrentQuest (Variables|Default|GetAC_QuestActor))))))
  (return (and (!= _outputpin -1) (== (.CurrentSubTask (Utilities|Struct|BreakS_QuestDynam (Utilities|Array|Get(acopy) (Variables|/Game/CompleteRPG/Blueprints/MapComponents/AC_QuestsHandler.AC_QuestsHandler_C|GetQuests _returnvalue) _outputpin))) 1))))