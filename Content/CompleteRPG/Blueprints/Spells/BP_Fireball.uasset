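; BP_Fireball is a spell projectile that damages attackable characters and explodes.
; On spawn, owner skills increase its radius and damage and reduce the energy cost drained from the caster.
; A forward line trace makes it home on a character's mesh, or fly without gravity otherwise.
; Sphere overlaps damage characters implementing BP_I_CanBeAttacked, excluding the owner, while other overlaps need a capsule trace hit to explode it.
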(event OnComponentBeginOverlap(Sphere)
  (params (OverlappedComponent :type Primitive%20Component%20Object%20Reference) (OtherActor :type Actor%20Object%20Reference) (OtherComp :type Primitive%20Component%20Object%20Reference) (OtherBodyIndex :type Integer) (bFromSweep :type Boolean) (SweepResult :type Hit%20Result%20Structure%20%28by%20ref%29))
  (bind _returnvalue (Transformation|GetActorLocation))
  ;[1 1 1] Overlap Object Event
  (bind _ascharacter (Utilities|Casting|CastToCharacter OtherActor)
    (:then
      (if (and (!= _ascharacter (Components|GetOwner)) (Utilities|DoesObjectImplementInterface _ascharacter "/Game/CompleteRPG/Blueprints/Other/Interfaces/BP_I_CanBeAttacked.BP_I_CanBeAttacked_C"))
        (Game|Damage|ApplyDamage _ascharacter (+ (Variables|Default|GetDamage) (.Value (Default|GetSkillValue (Actor|GetComponentbyClass (Components|GetOwner) "/Game/CompleteRPG/Blueprints/Skills/AC_Skills.AC_Skills_C") (Variables|Default|GetDamageSkill)))) 0 (Components|GetOwner))
        (Effects|SpawnEmitteratLocation "/Game/CompleteRPG/Blueprints/Weather/Particles/PS_Explosion.PS_Explosion" (Transformation|GetActorLocation))
        (Actor|DestroyActor)))
    (:CastFailed
      (bind _returnvalue_2 (Collision|CapsuleTraceByChannel _returnvalue _returnvalue 5e+01 5e+01 "TraceTypeQuery1" false 0 "None"))
      (if _returnvalue_2
        (Effects|SpawnEmitteratLocation "/Game/CompleteRPG/Blueprints/Weather/Particles/PS_Explosion.PS_Explosion" (Transformation|GetActorLocation))
        (Actor|DestroyActor)))))

(event Collision|EventActorBeginOverlap
  (params (OtherActor :type Actor%20Object%20Reference))
  (|CallParentFunction OtherActor))

(event EventBeginPlay
  (bind _returnvalue (Transformation|GetActorLocation))
  ;[1 1 1] Setup Events On Fireball Fired
  (Components|Sphere|SetSphereRadius (Variables|Default|GetSphere) (+ (Variables|Default|GetSphereRadius) (.Value (Default|GetSkillValue (Actor|GetComponentbyClass (Components|GetOwner) "/Game/CompleteRPG/Blueprints/Skills/AC_Skills.AC_Skills_C") (Variables|Default|GetRadiusSkill)))) true)
  (Default|RemoveEnergy (Actor|GetComponentbyClass (Components|GetOwner) "/Game/CompleteRPG/Blueprints/Player/AC_PlayerCharaacteristics.AC_PlayerCharaacteristics_C") (- (Variables|Default|GetCost) (.Value (Default|GetSkillValue (Actor|GetComponentbyClass (Components|GetOwner) "/Game/CompleteRPG/Blueprints/Skills/AC_Skills.AC_Skills_C") (Variables|Default|GetEnergySkill)))))
  (bind (_outhit _returnvalue_2) (Collision|LineTraceByChannel _returnvalue (+ _returnvalue (* (Transformation|GetActorForwardVector) 1.5e+04)) "TraceTypeQuery1" false 0 "None"))
  (if _returnvalue_2
    (bind _ascharacter (Utilities|Casting|CastToCharacter (.HitActor (Collision|BreakHitResult _outhit)))
      (:then
        (Variables|/Script/Engine.ProjectileMovementComponent|SetHomingTargetComponent (Variables|Default|GetProjectileMovement) (Variables|/Script/Engine.Character|GetMesh _ascharacter)))
      (:CastFailed
        (Variables|/Script/Engine.ProjectileMovementComponent|SetProjectileGravityScale (Variables|Default|GetProjectileMovement) 0.0)))
    (else
      (Variables|/Script/Engine.ProjectileMovementComponent|SetProjectileGravityScale (Variables|Default|GetProjectileMovement) 0.0))))

(event EventTick
  (params (DeltaSeconds :type Float%20%28single-precision%29))
  (|CallParentFunction DeltaSeconds))

(fn ConstructionScript
  (|CallParentFunction))