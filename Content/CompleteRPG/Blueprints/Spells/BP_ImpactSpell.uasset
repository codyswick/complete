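; Channeled impact spell actor that repeatedly knocks back and damages characters within a sphere around it.
; On begin play it sizes the sphere using the owner's radius skill, attaches a fire sound and starts a looping pulse timer.
; Each pulse drains skill-reduced energy from the owner, launches others along the owner's forward vector and applies skill-boosted magical or physical damage.
; The sound fades out when the spell is destroyed.
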(event Custom|DamageOverlaped
  (Default|RemoveEnergy (Actor|GetComponentbyClass (Components|GetOwner) "/Game/CompleteRPG/Blueprints/Player/AC_PlayerCharaacteristics.AC_PlayerCharaacteristics_C") (- (Variables|Default|GetCost) (.Value (Default|GetSkillValue (Actor|GetComponentbyClass (Components|GetOwner) "/Game/CompleteRPG/Blueprints/Skills/AC_Skills.AC_Skills_C") (Variables|Default|GetEnergySkill)))))
  (for _array_element (Variables|Default|GetCharactersArray)
    (Variables|Default|SetCurrent%20Character _array_element)
    (if (!= _array_element (Components|GetOwner))
      (Utilities|IsValid (Variables|Default|GetCurrent%20Character)
        (:Is%20Valid
          (Character|LaunchCharacter (Variables|Default|GetCurrent%20Character) (* (Transformation|GetActorForwardVector (Components|GetOwner)) 5e+03) true false)
          (Utilities|IsValid (Actor|GetComponentbyClass (Variables|Default|GetCurrent%20Character) "/Game/CompleteRPG/Blueprints/Player/AC_PlayerCharaacteristics.AC_PlayerCharaacteristics_C")
            (:Is%20Valid
              (bind _ascharacter (Utilities|Casting|CastToCharacter (Components|GetOwner)))
              (Default|RemoveHealth (Actor|GetComponentbyClass (Variables|Default|GetCurrent%20Character) "/Game/CompleteRPG/Blueprints/Player/AC_PlayerCharaacteristics.AC_PlayerCharaacteristics_C") (+ (Variables|Default|GetDamage) (.Value (Default|GetSkillValue (Actor|GetComponentbyClass (Components|GetOwner) "/Game/CompleteRPG/Blueprints/Skills/AC_Skills.AC_Skills_C") (Variables|Default|GetDamageSkill)))) true _ascharacter))))
        (:Is%20Not%20Valid
          (Utilities|Array|RemoveItem (Variables|Default|GetCharactersArray) (Variables|Default|GetCurrent%20Character)))))))

(event Custom|OnDestroyed_Event_0
  (params (DestroyedActor :type Actor%20Object%20Reference))
  (Audio|Components|Audio|FadeOut (stale EventBeginPlay _returnvalue) 1.0 0.0 :!class /Script/Engine.AudioComponent))

(event EventBeginPlay
  (Components|Sphere|SetSphereRadius (Variables|Default|GetSphere) (+ (Variables|Default|GetSphereRadius) (.Value (Default|GetSkillValue (Actor|GetComponentbyClass (Components|GetOwner) "/Game/CompleteRPG/Blueprints/Skills/AC_Skills.AC_Skills_C") (Variables|Default|GetRadiusSkill)))) true)
  (|CallParentFunction)
  (Utilities|Time|SetTimerbyEvent (delegate Custom|DamageOverlaped) 0.2 true)
  (bind _returnvalue (Audio|SpawnSoundAttached "/Game/CompleteRPG/Sounds/S_fire2.S_fire2" (Variables|Default|GetParticleSystem) "None" "0, 0, 0" "0, 0, 0" "KeepRelativeOffset" false 0.15 1.0 0.0 0 0 false))
  (EventDispatchers|AssignOnDestroyed (delegate Custom|OnDestroyed_Event_0)))

(event EventTick
  (params (DeltaSeconds :type Float%20%28single-precision%29))
  (|CallParentFunction DeltaSeconds))

(fn ConstructionScript
  (|CallParentFunction))