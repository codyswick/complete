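; Travel NPC that sells map travel through a timed conversation decision.
; After conversation setup, it filters Maps by the player's AC_ExpSystem level and builds priced options plus Quit, categorized by affordability via AC_MoneySystem.
; A choice charges the player, shows a loading screen, saves and opens the level after a short delay; insufficient funds triggers a refusal line that ends the conversation.
; Travel is free when the price is zero or no money component exists.
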(event EventBeginPlay
  (|CallParentFunction) ; This node is disabled and will not be called.\nDrag off pins to build functionality.
)

(event Collision|EventActorBeginOverlap
  (params (OtherActor :type Actor%20Object%20Reference)))

(event EventOnDecisionMade
  (params (DecisionIndex :type Integer) (ChosenOptionIndex :type Integer))
  (bind _returnvalue (- ChosenOptionIndex 1))
  (bind _leveledmaps (Variables|Default|GetLeveledMaps))
  (bind _importantdialogues (Variables|Default|GetImportantDialogues))
  (bind (_dialogueinfo _camera) (CallFunction|GetDialogueInfo _importantdialogues 1))
  (bind _output (Utilities|Array|Get(acopy) _leveledmaps _returnvalue))
  (bind (_displayname _filename _minlevel _price) (Utilities|Struct|BreakS_TravelMap _output))
  ;[1 1 1] Travel To The Choosed Map
  (switch int DecisionIndex
    (:0
      (if (== ChosenOptionIndex (Utilities|Array|Length (Variables|Default|GetOptions)))
        (CallFunction|EndConversation)
        (else
          (bind _result (CallFunction|PayforTravel _price))
          (if _result
            (bind _returnvalue_2 (UserInterface|CreateWidget "/Game/CompleteRPG/UI/Widgets/Menu/WB_LoadingScreen.WB_LoadingScreen_C"))
            (UserInterface|Viewport|AddtoViewport _returnvalue_2 0)
            (CallFunction|SaveGame (Variables|Default|GetPlayerChar))
            (Utilities|FlowControl|Delay 1.1)
            (Game|OpenLevel(byName) _filename)
            (else
              (CallFunction|AddCustomImportantDialogue 0 _dialogueinfo _camera))))))))

(event EventOnDialogueEnd
  (params (Index :type Integer))
  (switch int Index
    (:0
      (CallFunction|EndConversation))))

(event EventTick
  (params (DeltaSeconds :type Float%20%28single-precision%29)))

(event EventAfterConversationSetup
  (bind _importantdialogues (Variables|Default|GetImportantDialogues))
  (bind (_dialogueinfo _camera) (CallFunction|GetDialogueInfo _importantdialogues))
  (Utilities|Array|Clear (Variables|Default|GetOptions))
  (Utilities|Array|Clear (Variables|Default|GetLeveledMaps))
  (CallFunction|FilterPermissedLevels)
  (CallFunction|GenerateOptions)
  (CallFunction|AddDecision 0 (Utilities|Struct|MakeS_OptionInfo _dialogueinfo (Variables|Default|GetOptions) false 15) _camera))

(fn ConstructionScript
  (|CallParentFunction))

(fn FilterPermissedLevels
  (for _array_element (Variables|Default|GetMaps)
    (if (<= (.MinLevel (Utilities|Struct|BreakS_TravelMap _array_element)) (Variables|/Game/CompleteRPG/Blueprints/MapComponents/PlayerState/AC_ExpSystem.AC_ExpSystem_C|GetCurrentLevel (Actor|GetComponentbyClass (Variables|Default|GetPlayerChar) "/Game/CompleteRPG/Blueprints/MapComponents/PlayerState/AC_ExpSystem.AC_ExpSystem_C")))
      (Utilities|Array|Add (Variables|Default|GetLeveledMaps) _array_element))))

(fn GenerateOptions
  (bind _playerchar (Variables|Default|GetPlayerChar))
  (bind _returnvalue (Actor|GetComponentbyClass _playerchar "/Game/CompleteRPG/Blueprints/MapComponents/PlayerState/AC_MoneySystem.AC_MoneySystem_C"))
  (for _array_element (Variables|Default|GetLeveledMaps)
    (Utilities|IsValid _returnvalue
      (:Is%20Valid
        (bind _result (Default|HaveMoney? _returnvalue (Math|Conversions|ToFloat(Integer) (.Price (Utilities|Struct|BreakS_TravelMap _array_element))))))
      (:Is%20Not%20Valid
        _))
    (Utilities|Array|Add (Variables|Default|GetOptions) (Utilities|Struct|MakeS_DialogueOption (Utilities|Text|FormatText "{Name} : {Price}" (Utilities|Text|ToText(Name) (.DisplayName (Utilities|Struct|BreakS_TravelMap _array_element))) (.Price (Utilities|Struct|BreakS_TravelMap _array_element))) 0 (select _result "NewEnumerator0" "NewEnumerator3"))))
  (Utilities|Array|Add (Variables|Default|GetOptions) (Utilities|Struct|MakeS_DialogueOption "Quit" 0 "NewEnumerator0")))

(fn PayforTravel
  (params (Price :type Integer))
  (bind _returnvalue (Math|Conversions|ToFloat(Integer) Price))
  (bind _playerchar (Variables|Default|GetPlayerChar))
  (bind _returnvalue_2 (Actor|GetComponentbyClass _playerchar "/Game/CompleteRPG/Blueprints/MapComponents/PlayerState/AC_MoneySystem.AC_MoneySystem_C"))
  (if (> Price 0)
    (Utilities|IsValid _returnvalue_2
      (:Is%20Valid
        (bind _result (Default|HaveMoney? _returnvalue_2 _returnvalue))
        (if _result
          (Default|RemoveMoney _returnvalue_2 _returnvalue)
          (Audio|PlaySound2D (Variables|Default|GetMoneySound) 1.0 1.0 0.0 0 0)
          (return true)
          (else
            (return false))))
      (:Is%20Not%20Valid
        (return true)))
    (else
      (return true))))